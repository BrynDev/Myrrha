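; Player character Blueprint for Myrrha that adds the HUD and loss overlay, sets pause and game-over menu classes, and triggers a damage vignette.
; Holding left mouse or gamepad left face button creates an aiming spline when fruit can be thrown; releasing destroys it.
; Each tick predicts the projectile path from the throw transform and speed, then rebuilds spline mesh segments along it at fixed intervals to preview the arc.
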(event EventBeginPlay
  (bind _returnvalue (UserInterface|CreateWidget "/Game/UI/BP_InGameHUD.BP_InGameHUD_C"))
  (UserInterface|Viewport|AddtoViewport _returnvalue 0)
  (bind _returnvalue_2 (UserInterface|CreateWidget "/Game/UI/BP_Overlay_Loss.BP_Overlay_Loss_C"))
  (UserInterface|Viewport|AddtoViewport _returnvalue_2 0))

(event EventTick
  (params (DeltaSeconds :type Float%20%28single-precision%29))
  (Throwing|DrawPredictionSpline))

(event EventShowDamageOverlay
  (Default|CallTriggerVignette))

(event Input|GamepadEvents|GamepadFaceButtonLeft
  (params (Key :type Key%20Structure :default "None"))
  (:Pressed
    (if (Class|MyrrhaCharacter|CanThrowFruit)
      (Throwing|CreatePredictionSpline)))
  (:Released
    (Throwing|DestroyPredictionSpline)))

(event Input|MouseEvents|LeftMouseButton
  (params (Key :type Key%20Structure :default "None"))
  (:Pressed
    (if (Class|MyrrhaCharacter|CanThrowFruit)
      (Throwing|CreatePredictionSpline)))
  (:Released
    (Throwing|DestroyPredictionSpline)))

(fn ConstructionScript
  (Variables|Default|Setm_PauseMenuClass "/Game/UI/BP_PauseMenu.BP_PauseMenu_C")
  (Variables|Default|Setm_GameOverMenuClass "/Game/UI/BP_GameOverMenu.BP_GameOverMenu_C"))

(fn CreatePredictionSpline
  (bind _returnvalue (AddComponent|AddSplineComponent false))
  (Variables|Throwing|SetPredictionSpline _returnvalue)
  (Rendering|SetActorHiddenInGame false))

(fn DestroyPredictionSpline
  (bind _predictionspline (Variables|Throwing|GetPredictionSpline)
    (:then
      (Components|DestroyComponent _predictionspline)
      (Variables|Throwing|SetPredictionSpline 0)
      (Throwing|DestroyPredictionMeshes))
    (:else)))

(fn DestroyPredictionMeshes
  (for _array_element (Variables|Throwing|GetPredictionSplineMeshes)
    (Components|DestroyComponent _array_element))
  (Utilities|Array|Clear (Variables|Throwing|GetPredictionSplineMeshes)))

(fn DrawPredictionSpline
  (Utilities|PredictionSplineValid?
    (:Is%20Valid
      (Utilities|FlowControl|Sequence
        (:then_0
          (bind _outpathpositions (Class|GameplayStatics|BlueprintPredictProjectilePathbyTraceChannel (Utilities|ThrowLocation) (Utilities|ThrowVelocity) false 1e+02 "ECC_WorldDynamic" false (Utilities|Array|MakeArray self) "None"))
          (Spline|SetSplinePoints (Variables|Throwing|GetPredictionSpline) _outpathpositions "World" true)
          (Throwing|DestroyPredictionMeshes))
        (:then_1
          (for _index (range 0 (Math|Float|Truncate (/ (Spline|GetSplineLength (Variables|Throwing|GetPredictionSpline)) 1e+02)))
            (LocalVariables|SetIndex _index)
            (bind _returnvalue (AddComponent|AddSplineMeshComponent true))
            (Utilities|Array|Add (Variables|Throwing|GetPredictionSplineMeshes) _returnvalue)
            (SplineMesh|SetStartandEnd _returnvalue (Spline|GetLocationatDistanceAlongSpline (Variables|Throwing|GetPredictionSpline) (* (LocalVariables|GetIndex) 1e+02) "World") (Math|Vector|ClampVectorSize (Spline|GetTangentatDistanceAlongSpline (Variables|Throwing|GetPredictionSpline) (* (LocalVariables|GetIndex) 1e+02) "World") 0.0 1e+02) (Spline|GetLocationatDistanceAlongSpline (Variables|Throwing|GetPredictionSpline) (* (+ (LocalVariables|GetIndex) 1) 1e+02) "World") (Math|Vector|ClampVectorSize (Spline|GetTangentatDistanceAlongSpline (Variables|Throwing|GetPredictionSpline) (* (+ (LocalVariables|GetIndex) 1) 1e+02) "World") 0.0 1e+02) true :!class /Script/Engine.SplineMeshComponent)))))))